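; BP_NetPC is a networked player controller that creates and feeds the in-game overlay HUD.
; BeginPlay builds the overlay only on the Remote authority branch, fills in player ID, player name and server name, then plays its intro animation.
; AddSystemMessage appends a log-item widget to the overlay's system message list and scrolls to the end, seeded with an empty entry at startup.
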(event `self.ReceiveBeginPlay`
  (bind _ingameoverlaywidget (`self.InGameOverlayWidget`))
  ; Begin Play
  (`/Engine/EditorBlueprintResources/ActorMacros.Switch Has Authority`
    (:`Remote`
      (bind _returnvalue (`|CreateWidget` "/Game/Widgets/WG_InGameOverlay.WG_InGameOverlay_C" self))
      (bind _output_get (set `self.InGameOverlayWidget` _returnvalue))
      (`UserWidget.AddToViewport` _output_get 0)
      (`self.InitializeInGameOverlay` (`self.playerID`) (`self.playerName`) (`self.serverName`))
      (`UserWidget.PlayAnimation` _ingameoverlaywidget (`/Game/Widgets/WG_InGameOverlay.StartOverlay` _ingameoverlaywidget) 0.0 1 "Forward" 1.0 false)
      (`self.AddSystemMessage` " \n \n \n \n \n \n \n \n \n \n \n \n \n \n \n \n \n \n \n \n"))))

(event `self.InitializeInGameOverlay`
  (params (newPlayerID :type Integer) (newPlayerName :type String) (newServerName :type String))
  (bind _ingameoverlaywidget (`self.InGameOverlayWidget`))
  ; Initialize InGameOverlay
  (`TextBlock.SetText` (`/Game/Widgets/WG_InGameOverlay.TB_PlayerID` _ingameoverlaywidget) (`KismetTextLibrary.Conv_IntToText` newPlayerID))
  (`TextBlock.SetText` (`/Game/Widgets/WG_InGameOverlay.TB_PlayerName` _ingameoverlaywidget) (`KismetTextLibrary.Conv_StringToText` newPlayerName))
  (set `/Game/Widgets/WG_InGameOverlay.ServerName` newServerName _ingameoverlaywidget))

(event `self.AddSystemMessage`
  (params (newSysMsg :type String))
  (bind _vb_systemmessagelog (`/Game/Widgets/WG_InGameOverlay.VB_SystemMessageLog` (`self.InGameOverlayWidget`)))
  ; Add SystemMessage
  (bind _returnvalue (`|CreateWidget` "/Game/Widgets/WG_SysMsgLog_Item.WG_SysMsgLog_Item_C" null newSysMsg))
  (`PanelWidget.AddChild` _vb_systemmessagelog _returnvalue)
  (`ScrollBox.ScrollToEnd` _vb_systemmessagelog))

(fn `UserConstructionScript`)