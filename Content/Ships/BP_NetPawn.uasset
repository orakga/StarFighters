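; BP_NetPawn is a networked ship pawn that shows an on-screen label with the ship's ID and name.
; On BeginPlay, remote instances cache the WG_ShipLabel widget from the ShipLabel component, while the authority skips this; each path prints a debug message.
; SetLabel writes the ship ID and name into the cached widget, without checking that the reference is valid.
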(event `self.ReceiveBeginPlay`
  (`/Engine/EditorBlueprintResources/ActorMacros.Switch Has Authority`
    (:`Authority`
      (`KismetSystemLibrary.PrintString` "BP_NetPawn AUTHORITY: No Label Needed" true true (struct :`G` 0.984599 :`B` 1.0 :`A` 1.0) 4.0))
    (:`Remote`
      (bind _aswg_ship_label (cast `/Game/Widgets/WG_ShipLabel` (`WidgetComponent.GetUserWidgetObject` (`self.ShipLabel`)))
        (:`then`
          (set `self.ShipLabelWidget` _aswg_ship_label)
          (`KismetSystemLibrary.PrintString` "BP_NetPawn FOUND Ship Label" true true (struct :`R` 0.107666 :`G` 1.0 :`A` 1.0) 4.0))
        (:`CastFailed`
          (`KismetSystemLibrary.PrintString` "BP_NetPawn CANNOT FIND Ship Label" true true (struct :`R` 1.0 :`B` 0.026037 :`A` 1.0) 4.0))))))

(event `self.SetLabel`
  (params (shipID :type Integer) (shipName :type String))
  (bind _shiplabelwidget (`self.ShipLabelWidget`))
  ; Set Label ()
  (set `/Game/Widgets/WG_ShipLabel.ShipID` (`KismetStringLibrary.Conv_IntToString` shipID) _shiplabelwidget)
  (set `/Game/Widgets/WG_ShipLabel.ShipName` shipName _shiplabelwidget))

(fn `UserConstructionScript`)