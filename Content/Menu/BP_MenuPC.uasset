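; BP_MenuPC is the menu player controller that shows the main menu overlay and displays the player name and server IP.
; On BeginPlay it creates a WG_MainMenuOverlay widget for player controller 0, stores it and adds it to the viewport.
; The RegisterPlayerName and RegisterServerIP events write incoming values into the overlay's matching text fields.
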(event `self.ReceiveBeginPlay`
  (bind _returnvalue (`|CreateWidget` "/Game/Menu/WG_MainMenuOverlay.WG_MainMenuOverlay_C" (`GameplayStatics.GetPlayerController` 0)))
  (bind _output_get (set `self.MenuOverlayWidget` _returnvalue))
  (`UserWidget.AddToViewport` _output_get 0))

(event `self.RegisterPlayerName`
  (params (newPlayerName :type String))
  (`EditableTextBox.SetText` (`/Game/Menu/WG_MainMenuOverlay.PlayerName` (`self.MenuOverlayWidget`)) (`KismetTextLibrary.Conv_StringToText` newPlayerName)))

(event `self.RegisterServerIP`
  (params (newServerIP :type String))
  (`EditableTextBox.SetText` (`/Game/Menu/WG_MainMenuOverlay.ServerIP` (`self.MenuOverlayWidget`)) (`KismetTextLibrary.Conv_StringToText` newServerIP)))

(fn `UserConstructionScript`)